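; Short-lived spawner actor that fires a volley of projectiles at a target, then destroys itself.
; On BeginPlay it spawns a random number of ProjectileType actors at ShootPoint, passing along its owner and Target.
; Each gets a random speed and a random aim point in a thin horizontal box slightly above the target's origin, scattering the volley.
; The spawner's capsule ignores each spawned projectile when moving.
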(event `self.ReceiveBeginPlay`
  (bind _target (`self.Target`))
  (for _ (range (+ (`KismetMathLibrary.RandomIntegerInRange` 3 6) 1))
    (bind _returnvalue (`|SpawnActorFromClass` (`self.ProjectileType`) (`SceneComponent.K2_GetComponentToWorld` (`self.ShootPoint`)) "Undefined" "MultiplyWithRoot" (`self.GetOwner`) (`KismetMathLibrary.RandomFloatInRange` 100.0 400.0) 0.0 _target (`KismetMathLibrary.RandomPointInBoundingBox` (+ (`self.K2_GetActorLocation` _target) (0.0 0.0 50.0)) (200.0 200.0 1.0)) null))
    (`PrimitiveComponent.IgnoreActorWhenMoving` (`self.CapsuleComponent`) _returnvalue true))
  (`self.K2_DestroyActor`))

(fn `UserConstructionScript`)